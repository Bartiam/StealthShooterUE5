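; Gameplay ability that opens and closes the player's inventory screen in the stealth shooter.
; On activation it adds the HUD's inventory widget to the viewport, switches to Game and UI input, and shows the cursor.
; A WaitInputPress task makes the next press close the screen, end the ability and restore game-only input.
; Closing also unbinds the inventory's OnGetKeyFromInventory event and clears its item-choice flag.
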(event Ability|EventActivateAbility
  (bind _inventorywidget (CallFunction|GetInventoryWidget))
  (bind _asssplayer_base (Utilities|Casting|CastToSSPlayer_Base (Ability|GetAvatarActorfromActorInfo)))
  (Variables|Default|SetCurrentCharacter _asssplayer_base)
  (Ability|Tasks|WaitInputPress false
    (:then
      (UserInterface|Viewport|AddtoViewport _inventorywidget 0)
      (Input|SetInputModeGameandUI (CallFunction|GetOwnerController) _inventorywidget "DoNotLock" false false)
      (Variables|/Script/Engine.PlayerController|SetbShowMouseCursor (CallFunction|GetOwnerController) true))
    (:OnPress
      (Widget|RemovefromParent _inventorywidget)
      (Ability|EndAbility)
      (Input|SetInputModeGameOnly (CallFunction|GetOwnerController) false)
      (Variables|/Script/Engine.PlayerController|SetbShowMouseCursor (CallFunction|GetOwnerController) false)
      (bind _returnvalue (Class|SSPlayerBase|GetPlayerInventory (Variables|Default|GetCurrentCharacter)))
      (EventDispatchers|UnbindallEventsfromOnGetKeyfromInventory _returnvalue)
      (Variables|/Script/StealthShooterUE5.SS_InventoryComponent|SetbIsNeedToChooseItem _returnvalue false))))

(fn GetInventoryWidget
  (bind _returnvalue (Class|SSCharacterBase|GetOwnerPlayerController (Variables|Default|GetCurrentCharacter)))
  (bind _returnvalue_2 (Class|SSPlayerControllerBase|GetCurrentHUD _returnvalue))
  (bind _returnvalue_3 (Class|SSHUDBase|GetInventoryWidget _returnvalue_2))
  (return _returnvalue_3))

(fn GetOwnerController
  (bind _returnvalue (Class|SSCharacterBase|GetOwnerPlayerController (Variables|Default|GetCurrentCharacter)))
  (return _returnvalue))