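; Gameplay ability that makes the owning character crouch while its input is held.
; On activation it calls Crouch and applies GE_ChangeSpeed to the owner, while WaitInputRelease listens for release.
; On release it calls UnCrouch, ends the ability, then applies the same GE_ChangeSpeed effect again.
; The character comes from the avatar actor through a GetOwnerCharacterMessage call.
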(event Ability|EventActivateAbility
  (Ability|Tasks|WaitInputRelease false
    (:then
      (Character|Crouch (CallFunction|GetCurrentOwnerCharacter))
      (Ability|ApplyGameplayEffectToOwner "/Game/StealthShooter/Blueprints/PlayerCharacters/CharacterAbilities/GameplayEffects/GE_ChangeSpeed.GE_ChangeSpeed_C"))
    (:OnRelease
      (Character|UnCrouch (CallFunction|GetCurrentOwnerCharacter))
      (Ability|EndAbility)
      (Ability|ApplyGameplayEffectToOwner "/Game/StealthShooter/Blueprints/PlayerCharacters/CharacterAbilities/GameplayEffects/GE_ChangeSpeed.GE_ChangeSpeed_C"))))

(fn GetCurrentOwnerCharacter
  (bind _returnvalue (Class|CharacterInterface|GetOwnerCharacter(Message) (Ability|GetAvatarActorfromActorInfo)))
  (return _returnvalue))