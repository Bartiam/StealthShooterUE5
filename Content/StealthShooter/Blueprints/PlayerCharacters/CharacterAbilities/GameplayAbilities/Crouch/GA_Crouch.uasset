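; Gameplay ability that crouches the player character for as long as its input is held.
; On activation it applies a walk-and-crouch or plain crouch effect, depending on the Walk status tag, and sends Crouch through the owner's player message call.
; A WaitInputRelease task handles release, applying the walk or run effect by the same tag check, ending the ability, then calling UnCrouch.
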(event Ability|EventActivateAbility
  (Ability|Tasks|WaitInputRelease false
    (:then
      ;[1 1 1] Check gameplay tag "Walk" and apply gameplay effect to self
      (if (GameplayTags|HasMatchingGameplayTag (Ability|GetAbilitySystemComponent (Ability|GetAvatarActorfromActorInfo)) "(TagName=\"Character.Status.Walk\")")
        (Ability|ApplyGameplayEffectToOwner "/Game/StealthShooter/Blueprints/PlayerCharacters/CharacterAbilities/GE_WalkAndCrouch.GE_WalkAndCrouch_C")
        (else
          (Ability|ApplyGameplayEffectToOwner "/Game/StealthShooter/Blueprints/PlayerCharacters/CharacterAbilities/GameplayAbilities/Crouch/GE_Crouch.GE_Crouch_C")))
      (bind _returnvalue (Class|CharacterInterface|GetOwnerPlayer(Message) (Ability|GetAvatarActorfromActorInfo)))
      (Character|Crouch _returnvalue))
    (:OnRelease
      ;[1 1 1] Check gameplay tag "Walk" and apply gameplay effect to self
      (if (GameplayTags|HasMatchingGameplayTag (Ability|GetAbilitySystemComponent (Ability|GetAvatarActorfromActorInfo)) "(TagName=\"Character.Status.Walk\")")
        (Ability|ApplyGameplayEffectToOwner "/Game/StealthShooter/Blueprints/PlayerCharacters/CharacterAbilities/GameplayAbilities/Walk/GE_Walk.GE_Walk_C")
        (Ability|EndAbility)
        (else
          (Ability|ApplyGameplayEffectToOwner "/Game/StealthShooter/Blueprints/PlayerCharacters/CharacterAbilities/GameplayAbilities/Run/GE_Run.GE_Run_C")
          (Ability|EndAbility)))
      (bind _returnvalue_2 (Class|CharacterInterface|GetOwnerPlayer(Message) (Ability|GetAvatarActorfromActorInfo)))
      (Character|UnCrouch _returnvalue_2))))